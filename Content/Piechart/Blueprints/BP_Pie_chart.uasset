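; Pie chart actor that rebuilds its slices from a Values array in the construction script and on BeginPlay.
; FormatData normalizes the values to fractions of their sum, then UpdatePieChartData unregisters the old children and adds a flattened static mesh under Pie for each fraction.
; Each mesh gets a dynamic material instance with a random color and Start/Stop scalars from a running offset to define its slice.
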(event EventBeginPlay
  ;[1 1 1] if get data time is now
  (if true
    (CallFunction|UpdatePieChartData (Variables|Default|GetValues))))

(event Collision|EventActorBeginOverlap
  (params (OtherActor :type Actor%20Object%20Reference)))

(event EventTick
  (params (DeltaSeconds :type Float%20%28single-precision%29)))

(fn ConstructionScript
  (CallFunction|UpdatePieChartData (Variables|Default|GetValues)))

(fn FormatData
  (params (Values :type Array%20of%20Floats%20%28single-precision%29))
  (for _array_element Values
    (LocalVariables|SetSum (+ _array_element (LocalVariables|GetSum))))
  (for _array_element_2 Values
    (Utilities|Array|Add (LocalVariables|GetFormatedValues) (/ _array_element_2 (LocalVariables|GetSum))))
  (return (LocalVariables|GetFormatedValues)))

(fn CreateMaterialInstance
  (params (self2 :type Primitive%20Component%20Object%20Reference) (Start :type Float%20%28single-precision%29) (Stop :type Float%20%28single-precision%29))
  (bind _returnvalue (Rendering|Material|CreateDynamicMaterialInstance self2 0 "/Game/Piechart/Materials/Pie_Mat.Pie_Mat" :!class /Script/Engine.PrimitiveComponent))
  (Rendering|Material|SetVectorParameterValue _returnvalue "colorRGB" (Math|Color|MakeColor (Math|Random|RandomFloatinRange 0.0 1.0) (Math|Random|RandomFloatinRange 0.0 1.0) (Math|Random|RandomFloatinRange 0.0 1.0)) :!class /Script/Engine.MaterialInstanceDynamic)
  (Rendering|Material|SetScalarParameterValue _returnvalue "Start" Start :!class /Script/Engine.MaterialInstanceDynamic)
  (Rendering|Material|SetScalarParameterValue _returnvalue "Stop" (- 1.0 Stop) :!class /Script/Engine.MaterialInstanceDynamic))

(fn UpdatePieChartData
  (params (Values :type Array%20of%20Floats%20%28single-precision%29))
  (bind _pie (Variables|Default|GetPie))
  (bind _children (Components|GetChildrenComponents _pie false))
  (for _array_element _children
    (Class|JavascriptLibrary|UnregisterComponent _array_element))
  (Utilities|Array|Clear _children)
  (bind _output_get (Variables|Default|SetValues Values))
  (bind _formated_values (CallFunction|FormatData _output_get))
  (for _array_element_2 _formated_values
    (bind _returnvalue (AddComponent|AddStaticMeshComponent true (Math|Transform|MakeTransform "0, 0, 0" "0, 0, 0" "1,1,0.133484")))
    (Transformation|AttachComponentToComponent _returnvalue (Variables|Default|GetPie) "None" "SnapToTarget" "KeepRelative" "KeepRelative" true)
    (CallFunction|CreateMaterialInstance _returnvalue (LocalVariables|GetLastValue) (- (LocalVariables|GetLastValue) _array_element_2))
    (LocalVariables|SetLastValue (- (LocalVariables|GetLastValue) _array_element_2))))