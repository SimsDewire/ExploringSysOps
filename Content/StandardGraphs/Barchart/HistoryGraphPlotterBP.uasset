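; History bar chart actor that plots a rolling series of values as scaled static mesh bars along sized axes.
; Each new value spawns a bar from ValueTemplate at the front, shifts older bars along and removes those beyond BarCount.
; Bar heights are renormalized to the series maximum and BarMaxHeight on every update.
; UpdategraphData feeds in arrays, while Tick currently pushes random values at UpdateIntervalPerSec.
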(event EventBeginPlay)

(event EventTick
  (params (DeltaSeconds :type Float%20%28single-precision%29))
  (|ExecuteOnceEveryNSecond DeltaSeconds (Variables|Chart|GetUpdateIntervalPerSec))
  (CallFunction|UpdateNewValue (Math|Random|RandomFloatinRange 1e+01 1e+02))
  (Variables|Private|SetTimeElapsed 0.0))

(fn ConstructionScript
  (|CallParentFunction)
  (CallFunction|SetYLength (Variables|Default|GetBarMaxHeight)))

(fn UpdateNewValue
  (params (NewValue :type Float%20%28single-precision%29))
  (LocalVariables|SetNextValue NewValue)
  (CallFunction|SetYLength (Variables|Default|GetBarMaxHeight))
  (Utilities|FlowControl|Sequence
    (:then_0
      ;[1 1 1] Add and normalize the values already in history queue
      (|Addnewvalue)
      (bind _normalizedvalues (CallFunction|NormalizeValues (Variables|Private|GetHistoryValues) (Variables|Default|GetBarMaxHeight)))
      (LocalVariables|SetNormalizedValues _normalizedvalues))
    (:then_1
      (for (_array_element _array_index) (Variables|Private|GetHistoryValueTemplates) ; Update each bar value
        (LocalVariables|SetCurrentBar _array_element)
        (bind _barindex (|IsMoreBarsThanNeeded _array_index)
          (:True
            (|RemoveBar _barindex (LocalVariables|GetCurrentBar)))
          (:False
            (Utilities|FlowControl|Sequence
              (:then_0
                (if (> _barindex 0) ; Dont move the new first bar
                  (|AddOneBarOffsetToBar (LocalVariables|GetCurrentBar))))
              (:then_1
                (bind _returnvalue (Utilities|GetNewScale (Utilities|Array|Get(acopy) (LocalVariables|GetNormalizedValues) _array_index)))
                (Transformation|SetRelativeScale3D (LocalVariables|GetCurrentBar) _returnvalue) ; Set value of the new bar by scaling it
              )))))
      ;[1 1 1] Update the x axis to fit the amount of bars
      (CallFunction|SetXLength (* (Variables|Chart|GetBarCount) (- (Utilities|OneBarOffsetLocation) (Variables|Chart|GetBarOffset))))
      (return))))

(fn UpdategraphData
  (params (Values :type Array%20of%20Floats%20%28single-precision%29) (OverrideAll :type Boolean))
  (LocalVariables|SetInValues Values)
  (if OverrideAll ; Should we override the existing data?
    (Variables|Chart|SetBarCount (Utilities|Array|Length (LocalVariables|GetInValues)))
    (if (!= (Utilities|Array|Length (LocalVariables|GetInValues)) 0) ; Is there any data at all in the values array
      (for _array_element (LocalVariables|GetInValues) :!label _label
        (CallFunction|UpdateNewValue _array_element))
      (else
        (CallFunction|UpdateNewValue 0.0) ; Remove all data in the graph
      ))
    (else
      (goto _label)))
  (return))

(fn NormalizeValues
  (params (Values :type Array%20of%20Floats%20%28single-precision%29) (Roof :type Float%20%28single-precision%29))
  (LocalVariables|SetRoofTmp Roof)
  (bind _output_get (LocalVariables|SetNormalizedArray Values))
  (LocalVariables|SetMAX (.MaxValue (Math|Float|MaxOfFloatArray _output_get)))
  (for (_array_element _array_index) (LocalVariables|GetNormalizedArray)
    (Utilities|Array|SetArrayElem (LocalVariables|GetNormalizedArray) _array_index (* (/ _array_element (LocalVariables|GetMAX)) (LocalVariables|GetRoofTmp))))
  (return (LocalVariables|GetNormalizedArray)))