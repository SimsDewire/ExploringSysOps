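; OnOffButtonBP is an on/off indicator Blueprint that automatically switches its Sphere between two material states.
; Each Tick advances an accumulated timer by delta time plus a small random amount, making the blink irregular and frame-rate dependent.
; The timer modulo period X is compared with half of X, and the result drives the IsGreen scalar parameter on the Sphere's materials.
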(event EventTick
  (params (DeltaSeconds :type Float%20%28single-precision%29))
  (bind _x (Variables|Default|GetX))
  (bind _output_get (Variables|Default|SetTimeSinceCreation (+ DeltaSeconds (Math|Random|RandomFloatinRange 0.0 0.3) (Variables|Default|GetTimeSinceCreation))))
  (bind _output_get_2 (Variables|Default|SetIsOk (> (Math|Float|%(Float) _output_get _x) (/ _x 2.0))))
  (Rendering|Material|SetScalarParameterValueonMaterials (Variables|Default|GetSphere) "IsGreen" (Math|Conversions|ToFloat(Boolean) _output_get_2)))

(fn ConstructionScript)