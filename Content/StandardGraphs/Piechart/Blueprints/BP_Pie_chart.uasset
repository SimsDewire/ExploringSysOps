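; Pie chart actor that displays an array of values as proportional colored slices and can be picked up and dropped via attachment.
; It rebuilds in the construction script and on BeginPlay, removing old pieces and normalizing values by their sum.
; Each slice is a runtime-added copy of one mesh, with a dynamic material taking start, stop and color from the running total.
; Values lacking a color get a random one.
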(event EventBeginPlay
  (CallFunction|UpdatePieChartData (Variables|Pie|GetValues)) ; Make sure that the piechart is up to date when the game starts
)

(event EventDrop
  (Transformation|DetachFromActor "KeepWorld" "KeepWorld" "KeepWorld"))

(event EventPickup
  (params (AttachTo :type Scene%20Component%20Object%20Reference))
  (Transformation|AttachComponentToComponent AttachTo "None" "KeepWorld" "KeepWorld" "KeepWorld" true))

(fn ConstructionScript
  (CallFunction|UpdatePieChartData (Variables|Pie|GetValues)) ; Make the piechart update live in editor view
)

(fn FormatData
  (params (Values :type Array%20of%20Floats%20%28single-precision%29))
  (for _array_element Values
    (LocalVariables|SetSum (+ _array_element (LocalVariables|GetSum))))
  (for _array_element_2 Values
    (Utilities|Array|Add (LocalVariables|GetFormattedValues) (/ _array_element_2 (LocalVariables|GetSum))))
  (return (LocalVariables|GetFormattedValues)))

(fn CreateMaterialInstance
  (params (self2 :type Primitive%20Component%20Object%20Reference) (Start :type Float%20%28single-precision%29) (Stop :type Float%20%28single-precision%29) (Color :type Linear%20Color%20Structure))
  (Utilities|FlowControl|Sequence
    (:then_0
      ;[0.2464 1 0.4911] Setup local variables to be used everywhere =)
      (LocalVariables|SetStartValueLocal Start))
    (:then_1
      (bind _output_get (LocalVariables|SetStopValueLocal Stop))
      (LocalVariables|SetStopValueLocal (- 1.0 _output_get)))
    (:then_2
      (bind _returnvalue (Rendering|Material|CreateDynamicMaterialInstance self2 0 "/Game/StandardGraphs/Piechart/Materials/Pie_Mat.Pie_Mat" :!class /Script/Engine.PrimitiveComponent)) ; Creates a new material with the pie chart properties
      (LocalVariables|SetDynamicMaterial _returnvalue)
      (Utilities|FlowControl|Sequence
        (:then_0
          ;[0.2464 1 0.4911] Set material properties
          (Rendering|Material|SetScalarParameterValue (LocalVariables|GetDynamicMaterial) "Start" (LocalVariables|GetStartValueLocal) :!class /Script/Engine.MaterialInstanceDynamic))
        (:then_1
          (Rendering|Material|SetScalarParameterValue (LocalVariables|GetDynamicMaterial) "Stop" (LocalVariables|GetStopValueLocal) :!class /Script/Engine.MaterialInstanceDynamic))
        (:then_2
          (Rendering|Material|SetVectorParameterValue (LocalVariables|GetDynamicMaterial) "colorRGB" Color :!class /Script/Engine.MaterialInstanceDynamic))))))

(fn UpdatePieChartData
  (params (Values :type Array%20of%20Floats%20%28single-precision%29))
  (Utilities|DestroyAllPiePieces)
  (bind _output_get (Variables|Pie|SetValues Values))
  (bind _formatted_values (CallFunction|FormatData _output_get))
  (bind _targetarrayout (CallFunction|ResetPieColors _formatted_values))
  (for (_array_element _array_index) _targetarrayout
    (bind _decreasedvalue (Utilities|AddPiePiece (LocalVariables|GetLastValue) _array_element (Utilities|Array|Get(acopy) (Variables|Pie|GetValueColors) _array_index))
      (:ExecOut
        (LocalVariables|SetLastValue _decreasedvalue)))))

(fn ResetPieColors
  (params (TargetArrayIn :type Array%20of%20Floats%20%28single-precision%29))
  (bind _valuecolors (Variables|Pie|GetValueColors))
  (bind _returnvalue (Utilities|Array|Length _valuecolors))
  (LocalVariables|Setv TargetArrayIn)
  (LocalVariables|SetpreviousLength _returnvalue)
  (Utilities|Array|Resize _valuecolors (Math|Integer|Max(Integer) _returnvalue (Utilities|Array|Length TargetArrayIn)))
  (for _index (range (LocalVariables|GetpreviousLength) (Utilities|Array|LastIndex (Variables|Pie|GetValueColors)))
    (Utilities|Array|SetArrayElem (Variables|Pie|GetValueColors) _index (Utilities|Struct|MakeLinearColor (Math|Random|RandomFloatinRange 0.0 1.0) (Math|Random|RandomFloatinRange 0.0 1.0) (Math|Random|RandomFloatinRange 0.0 1.0) 1.0)))
  (return (LocalVariables|Getv)))